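; Turret actor (Torre) that continuously aims at its Target actor.
; Each Tick, look-at rotations split the aim across two components: Cabeza turns with zero pitch, while Pivote follows both yaw and pitch.
; Both snap directly to world rotations, with no interpolation or firing logic.
; An unconnected Cannon look-at chain remains in the graph but never runs.
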(event EventBeginPlay)

(event Collision|EventActorBeginOverlap
  (params (OtherActor :type Actor%20Object%20Reference)))

(event EventTick
  (params (DeltaSeconds :type Float%20%28single-precision%29))
  (bind _pivote (Variables|Default|GetPivote))
  (bind _cabeza (Variables|Default|GetCabeza))
  (bind _target (Variables|Default|GetTarget))
  (bind _returnvalue (Transformation|GetWorldLocation _pivote))
  (bind _returnvalue_2 (Transformation|GetActorLocation _target))
  (bind _returnvalue_3 (Transformation|GetWorldLocation _cabeza))
  (bind _returnvalue_4 (Math|Rotator|FindLookatRotation _returnvalue _returnvalue_2))
  (bind _returnvalue_5 (Math|Rotator|FindLookatRotation _returnvalue_3 _returnvalue_2))
  (bind (_roll _pitch _yaw) (Math|Rotator|BreakRotator _returnvalue_4))
  (bind (_roll_2 _pitch_2 _yaw_2) (Math|Rotator|BreakRotator _returnvalue_5))
  (Transformation|SetWorldRotation _cabeza (Math|Rotator|MakeRotator _roll_2 0.0 _yaw_2) false false)
  (Transformation|SetWorldRotation _pivote (Math|Rotator|MakeRotator 0.0 _pitch _yaw) false false))

(fn ConstructionScript)