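; InformacionJuegoActual is the Game Instance that holds the player's current XP and persists it between sessions through a GuardarPartida save object.
; LoadSaveGame copies saved XP into the instance when the slot exists, then re-saves it, or creates a new save from the current XP otherwise.
; SaveGame builds a fresh save object from the current XP and overwrites the slot.
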(fn LoadSaveGame
  (bind _returnvalue (SaveGame|DoesSaveGameExist (Variables|Default|GetSlotName)))
  (if _returnvalue
    (bind _returnvalue_2 (SaveGame|LoadGamefromSlot (Variables|Default|GetSlotName)))
    (bind _output_get (Variables|Default|SetSaverSubClass _returnvalue_2))
    (bind _asguardar_partida (Utilities|Casting|CastToGuardarPartida _output_get))
    (bind _asinformacion_juego_actual (Utilities|Casting|CastToInformacionJuegoActual (Game|GetGameInstance)))
    (Variables|InformacionJuegoActual_C|SetXP _asinformacion_juego_actual (Variables|/Game/Prototipos/GuardarPartida.GuardarPartida_C|GetXP _asguardar_partida))
    (SaveGame|SaveGametoSlot (Variables|Default|GetSaverSubClass) (Variables|Default|GetSlotName))
    (else
      (bind _returnvalue_3 (SaveGame|CreateSaveGameObject "/Game/Prototipos/GuardarPartida.GuardarPartida_C"))
      (bind _output_get_2 (Variables|Default|SetSaverSubClass _returnvalue_3))
      (bind _asguardar_partida_2 (Utilities|Casting|CastToGuardarPartida _output_get_2))
      (bind _asinformacion_juego_actual_2 (Utilities|Casting|CastToInformacionJuegoActual (Game|GetGameInstance)))
      (Variables|/Game/Prototipos/GuardarPartida.GuardarPartida_C|SetXP _asguardar_partida_2 (Variables|InformacionJuegoActual_C|GetXP _asinformacion_juego_actual_2))
      (SaveGame|SaveGametoSlot (Variables|Default|GetSaverSubClass) (Variables|Default|GetSlotName)))))

(fn SaveGame
  (bind _returnvalue (SaveGame|CreateSaveGameObject "/Game/Prototipos/GuardarPartida.GuardarPartida_C"))
  (bind _output_get (Variables|Default|SetSaverSubClass _returnvalue))
  (bind _asguardar_partida (Utilities|Casting|CastToGuardarPartida _output_get))
  (bind _asinformacion_juego_actual (Utilities|Casting|CastToInformacionJuegoActual (Game|GetGameInstance)))
  (Variables|/Game/Prototipos/GuardarPartida.GuardarPartida_C|SetXP _asguardar_partida (Variables|InformacionJuegoActual_C|GetXP _asinformacion_juego_actual))
  (SaveGame|SaveGametoSlot (Variables|Default|GetSaverSubClass) (Variables|Default|GetSlotName)))