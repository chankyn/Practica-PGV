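; SupportController runs the player's two targeted support strikes, Air and Nuke, against Bichos enemies.
; ActivarModoApoyo spawns a radius-scaled marker, which Tick moves to the cursor's object trace hit.
; A left click spawns effects, damages every Bichos within range by distance check and destroys those without health.
; It then removes the marker, sets that strike's cooldown end time and updates HUD widgets, showing the bar and disabling the button.
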(event EventTick
  (params (DeltaSeconds :type Float%20%28single-precision%29))
  ;[1 1 1] Seguir el movimiento del ratón durante el modo explosión
  (Utilities|FlowControl|Sequence
    (:then_1
      (if (Variables|Default|GetModo%20Apoyo)
        (Transformation|SetActorLocation (Variables|Default|GetCast%20Marker) (.Location (Collision|BreakHitResult (.HitResult (Class|PlayerController|GetHitResultUnderCursorforObjects (Game|GetPlayerController 0) (Utilities|Array|MakeArray "ObjectTypeQuery9") true)))) false false)))))

(event Input|MouseEvents|LeftMouseButton
  (params (Key :type Key%20Structure))
  ;[1 1 1] Control del evento para realizar el apoyo
  (:Pressed
    (if (Variables|Default|GetModo%20Apoyo)
      (CallFunction|ApoyoClick (.Location (Collision|BreakHitResult (.HitResult (Class|PlayerController|GetHitResultUnderCursorforObjects (Game|GetPlayerController 0) (Utilities|Array|MakeArray "ObjectTypeQuery9") true))))))))

(fn ConstructionScript)

(fn ActivarModoApoyo
  (params (Tipo%20Apoyo :type Integer))
  (bind _radio_air (Variables|Default|GetRadio%20Air))
  (bind _radio_nuke (Variables|Default|GetRadio%20Nuke))
  (bind _returnvalue (/ _radio_nuke 3.0))
  (bind _returnvalue_2 (/ _radio_air 3.0))
  ;[1 1 1] Activa el modo apoyo y "castea" el marker donde caerá el apoyo
  (Variables|Default|SetTipo%20Apoyo Tipo%20Apoyo)
  (Variables|Default|SetModo%20Apoyo true)
  (if (== Tipo%20Apoyo 0)
    (bind _returnvalue_3 (Game|SpawnActorfromClass "/Game/Blueprints/SupMarker.SupMarker_C" (Math|Transform|MakeTransform "0, 0, 0" "0, 0, 0" (Math|Vector|MakeVector _returnvalue_2 _returnvalue_2 _returnvalue_2)) "Undefined" 0 0))
    (Variables|Default|SetCast%20Marker _returnvalue_3)
    (elif (== Tipo%20Apoyo 1)
      (bind _returnvalue_4 (Game|SpawnActorfromClass "/Game/Blueprints/SupMarker.SupMarker_C" (Math|Transform|MakeTransform "0, 0, 0" "0, 0, 0" (Math|Vector|MakeVector _returnvalue _returnvalue _returnvalue)) "Undefined" 0 0))
      (Variables|Default|SetCast%20Marker _returnvalue_4))))

(fn ApoyoClick
  (params (Location :type Vector))
  ;[1 1 1] Si se está en "modo apoyo" del tipo "Air", genera una explosión y un sonido, realiza el daño a los enemigos y actualiza el HUD
  (if (Variables|Default|GetModo%20Apoyo)
    (if (== (Variables|Default|GetTipo%20Apoyo) 0)
      (Effects|SpawnEmitteratLocation "/Game/StarterContent/Particles/P_Explosion.P_Explosion" Location)
      (Audio|PlaySound2D "/Game/StarterContent/Audio/Explosion02.Explosion02" 1.0 1.0 0.0 0 0)
      (bind _outactors (Actor|GetAllActorsOfClass "/Game/Prototipos/Level/Bichos.Bichos_C"))
      (for _array_element _outactors
        (if (<= (Math|Vector|VectorLength (- (Transformation|GetActorLocation _array_element) Location)) (* (Variables|Default|GetRadio%20Air) 5e+01))
          (bind _output_get (Variables|/Game/Prototipos/Level/Bichos.Bichos_C|SetHealth _array_element (- (Variables|/Game/Prototipos/Level/Bichos.Bichos_C|GetHealth _array_element) (Variables|Default|GetDaño%20Air))))
          (if (<= _output_get 0.0)
            (Actor|DestroyActor _array_element))))
      (CallFunction|DesactivarModoApoyo)
      (bind _output_get_2 (Variables|Default|SetCDEnd%20Air (+ (Utilities|Time|GetTimeSeconds) (Variables|Default|GetConstant%20CD%20Air))))
      (bind _foundwidgets (Widget|GetAllWidgetsOfClass "/Game/Prototipos/Widget/HUDPrincipal/HUD.HUD_C" false))
      (for _array_element_2 _foundwidgets
        (Widget|SetVisibility (Variables|/Game/Prototipos/Widget/HUDPrincipal/HUD.HUD_C|GetBarra_CD_Air _array_element_2) "Visible")
        (Variables|/Game/Prototipos/Widget/HUDPrincipal/HUD.HUD_C|SetCD_Air _array_element_2 _output_get_2)
        (Widget|SetIsEnabled (Variables|/Game/Prototipos/Widget/HUDPrincipal/HUD.HUD_C|GetButton_AirSup _array_element_2) false))
      (elif (== (Variables|Default|GetTipo%20Apoyo) 1)
        ;[1 1 1] Si se está en "modo apoyo" del tipo "Nuke", genera una explosión y un sonido, realiza el daño a los enemigos y actualiza el HUD
        (Effects|SpawnEmitteratLocation "/Game/StarterContent/InfinityBladeEffects/Effects/FX_Monsters/FX_Monster_Gruntling/Bomber/P_FireBombExplosion.P_FireBombExplosion" Location)
        (Audio|PlaySound2D "/Game/StarterContent/Audio/Explosion01.Explosion01" 1.0 1.0 0.0 0 0)
        (bind _outactors_2 (Actor|GetAllActorsOfClass "/Game/Prototipos/Level/Bichos.Bichos_C"))
        (for _array_element_3 _outactors_2
          (if (<= (Math|Vector|VectorLength (- (Transformation|GetActorLocation _array_element_3) Location)) (* (Variables|Default|GetRadio%20Nuke) 2e+01))
            (bind _output_get_3 (Variables|/Game/Prototipos/Level/Bichos.Bichos_C|SetHealth _array_element_3 (- (Variables|/Game/Prototipos/Level/Bichos.Bichos_C|GetHealth _array_element_3) (Variables|Default|GetDaño%20Nuke))))
            (if (<= _output_get_3 0.0)
              (Actor|DestroyActor _array_element_3))))
        (CallFunction|DesactivarModoApoyo)
        (bind _output_get_4 (Variables|Default|SetCDEnd%20Nuke (+ (Utilities|Time|GetTimeSeconds) (Variables|Default|GetConstant%20CD%20Nuke))))
        (bind _foundwidgets_2 (Widget|GetAllWidgetsOfClass "/Game/Prototipos/Widget/HUDPrincipal/HUD.HUD_C" false))
        (for _array_element_4 _foundwidgets_2
          (Widget|SetVisibility (Variables|/Game/Prototipos/Widget/HUDPrincipal/HUD.HUD_C|GetBarra_CD_Nuke _array_element_4) "Visible")
          (Variables|/Game/Prototipos/Widget/HUDPrincipal/HUD.HUD_C|SetCD_Nuke _array_element_4 _output_get_4)
          (Widget|SetIsEnabled (Variables|/Game/Prototipos/Widget/HUDPrincipal/HUD.HUD_C|GetButton_NukeSup _array_element_4) false))))))

(fn DesactivarModoApoyo
  (bind _cast_marker (Variables|Default|GetCast%20Marker))
  ;[1 1 1] Desactiva el modo apoyo y elimina el "marker
  (Variables|Default|SetModo%20Apoyo false)
  (if (Utilities|IsValid _cast_marker)
    (Actor|DestroyActor _cast_marker)))