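; Tower targeting test Blueprint that turns a turret to face an actor inside its range trigger.
; Begin overlap stores any entering actor as the target and locks on; end overlap by any actor clears the lock.
; While locked, Tick splits the look-at rotation: Cabeza takes yaw and roll with zero pitch, while Pivote takes pitch and yaw.
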(event OnComponentBeginOverlap(TriggerRangoTorre)
  (params (OverlappedComponent :type Primitive%20Component%20Object%20Reference) (OtherActor :type Actor%20Object%20Reference) (OtherComp :type Primitive%20Component%20Object%20Reference) (OtherBodyIndex :type Integer) (bFromSweep :type Boolean) (SweepResult :type Hit%20Result%20Structure%20%28by%20ref%29))
  ;[1 1 1] TargetBloqueado a True cuando entra un enemigo al rango de la torre.
  (Variables|Default|SetTarget OtherActor)
  (Variables|Default|SetTargetBloqueado true))

(event OnComponentEndOverlap(TriggerRangoTorre)
  (params (OverlappedComponent :type Primitive%20Component%20Object%20Reference) (OtherActor :type Actor%20Object%20Reference) (OtherComp :type Primitive%20Component%20Object%20Reference) (OtherBodyIndex :type Integer))
  ;[1 1 1] TargetBloqeado a False cuando sale el target actual del rango de la torre.
  (Variables|Default|SetTargetBloqueado false))

(event EventTick
  (params (DeltaSeconds :type Float%20%28single-precision%29))
  (bind _pivote (Variables|Default|GetPivote))
  (bind _cabeza (Variables|Default|GetCabeza))
  (bind _target (Variables|Default|GetTarget))
  (bind _returnvalue (Transformation|GetWorldLocation _pivote))
  (bind _returnvalue_2 (Transformation|GetActorLocation _target))
  (bind _returnvalue_3 (Transformation|GetWorldLocation _cabeza))
  (bind _returnvalue_4 (Math|Rotator|FindLookatRotation _returnvalue _returnvalue_2))
  (bind _returnvalue_5 (Math|Rotator|FindLookatRotation _returnvalue_3 _returnvalue_2))
  (bind (_roll _pitch _yaw) (Math|Rotator|BreakRotator _returnvalue_4))
  (bind (_roll_2 _pitch_2 _yaw_2) (Math|Rotator|BreakRotator _returnvalue_5))
  (if (Variables|Default|GetTargetBloqueado)
    (Transformation|SetWorldRotation _cabeza (Math|Rotator|MakeRotator _roll_2 0.0 _yaw_2) false false)
    (Transformation|SetWorldRotation _pivote (Math|Rotator|MakeRotator 0.0 _pitch _yaw) false false)))

(fn ConstructionScript)