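; Level 1 wave spawner actor that spawns four types of Bichito AI enemies at its own location.
; SpawnBichos advances the wave up to a total, then runs chained delayed loops, one type after another, sized by per-wave count arrays.
; Tick uses a Delay as a one-second countdown; at zero it re-enters the spawn chain after the increment, resetting the timer without advancing the wave.
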(event Custom|SpawnBichos
  (if (< (Variables|Default|GetOleadaActual) (Variables|Default|GetTotalOleadas))
    (Variables|Default|SetOleadaActual (+ (Variables|Default|GetOleadaActual) 1))
    (Variables|Default|SetTimeOleada 30)
    (Utilities|ForLoopwithDelay 0 (Utilities|Array|Get(acopy) (Variables|Default|GetBichosT1) (Variables|Default|GetOleadaActual)) 0.5
      (:LoopBody
        (AI|SpawnAIFromClass "/Game/Prototipos/Level/Bichito1.Bichito1_C" 0 (Transformation|GetActorLocation) "0, 0, 0" false))
      (:Completed
        (Utilities|ForLoopwithDelay 0 (Utilities|Array|Get(acopy) (Variables|Default|GetBichosT2) (Variables|Default|GetOleadaActual)) 0.5
          (:LoopBody
            (AI|SpawnAIFromClass "/Game/Prototipos/Level/Bichito2.Bichito2_C" 0 (Transformation|GetActorLocation) "0.000000, 0, 0" false))
          (:Completed
            (Utilities|ForLoopwithDelay 0 (Utilities|Array|Get(acopy) (Variables|Default|GetBichosT3) (Variables|Default|GetOleadaActual)) 0.5
              (:LoopBody
                (AI|SpawnAIFromClass "/Game/Prototipos/Level/Bichito3.Bichito3_C" 0 (Transformation|GetActorLocation) "0, 0, 0" false))
              (:Completed
                (Utilities|ForLoopwithDelay 0 (Utilities|Array|Get(acopy) (Variables|Default|GetBichosT4) (Variables|Default|GetOleadaActual)) 0.5
                  (:LoopBody
                    (AI|SpawnAIFromClass "/Game/Prototipos/Level/Bichito4.Bichito4_C" 0 (Transformation|GetActorLocation) "0, 0, 0" false)))))))))))

(event EventTick
  (params (DeltaSeconds :type Float%20%28single-precision%29))
  (Utilities|FlowControl|Delay 1.0)
  (if (<= (Variables|Default|GetTimeOleada) 0)
    (Variables|Default|SetTimeOleada 30)
    (Utilities|ForLoopwithDelay 0 (Utilities|Array|Get(acopy) (Variables|Default|GetBichosT1) (Variables|Default|GetOleadaActual)) 0.5
      (:LoopBody
        (AI|SpawnAIFromClass "/Game/Prototipos/Level/Bichito1.Bichito1_C" 0 (Transformation|GetActorLocation) "0, 0, 0" false))
      (:Completed
        (Utilities|ForLoopwithDelay 0 (Utilities|Array|Get(acopy) (Variables|Default|GetBichosT2) (Variables|Default|GetOleadaActual)) 0.5
          (:LoopBody
            (AI|SpawnAIFromClass "/Game/Prototipos/Level/Bichito2.Bichito2_C" 0 (Transformation|GetActorLocation) "0.000000, 0, 0" false))
          (:Completed
            (Utilities|ForLoopwithDelay 0 (Utilities|Array|Get(acopy) (Variables|Default|GetBichosT3) (Variables|Default|GetOleadaActual)) 0.5
              (:LoopBody
                (AI|SpawnAIFromClass "/Game/Prototipos/Level/Bichito3.Bichito3_C" 0 (Transformation|GetActorLocation) "0, 0, 0" false))
              (:Completed
                (Utilities|ForLoopwithDelay 0 (Utilities|Array|Get(acopy) (Variables|Default|GetBichosT4) (Variables|Default|GetOleadaActual)) 0.5
                  (:LoopBody
                    (AI|SpawnAIFromClass "/Game/Prototipos/Level/Bichito4.Bichito4_C" 0 (Transformation|GetActorLocation) "0, 0, 0" false)))))))))
    (else
      (Variables|Default|SetTimeOleada (- (Variables|Default|GetTimeOleada) 1)))))

(fn ConstructionScript)