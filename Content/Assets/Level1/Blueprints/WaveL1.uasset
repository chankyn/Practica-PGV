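; WaveL1 is a wave spawner, apparently for Level 1, that spawns Bichito actors at its Cube's transform.
; Tick counts TimeOleada down once per frame, printing it, then resets it and calls SpawnBichitos, so wave timing depends on frame rate.
; SpawnBichitos reads the Bichito1 count from BichosT1 at OleadaActual, then advances that index with no bounds check.
; Loops for Bichito2 to Bichito4 exist but are unconnected and never run.
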(event EventBeginPlay)

(event EventTick
  (params (DeltaSeconds :type Float%20%28single-precision%29))
  (if (<= (Variables|Default|GetTimeOleada) 0)
    (Variables|Default|SetTimeOleada 30)
    (CallFunction|SpawnBichitos)
    (else
      (bind _output_get (Variables|Default|SetTimeOleada (- (Variables|Default|GetTimeOleada) 1)))
      (Development|PrintText (Utilities|Text|ToText(Integer) _output_get)))))

(fn ConstructionScript)

(fn SpawnBichitos
  (for _index (range 0 (Utilities|Array|Get(acopy) (Variables|Default|GetBichosT1) (Variables|Default|GetOleadaActual)))
    (Game|SpawnActorfromClass "/Game/Prototipos/Level/Bichito1.Bichito1_C" (Transformation|GetWorldTransform (Variables|Default|GetCube)) "Undefined" 0 0)
    (Development|PrintText "Hello"))
  (Variables|Default|SetOleadaActual (+ (Variables|Default|GetOleadaActual) 1)))