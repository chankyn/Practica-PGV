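; Automatic turret cannon that finds actors tagged "Enemigo" within Alcance and fires Missile actors at them.
; A looping BuscarTarget timer sphere-traces for a target and opens a Tick gate.
; Tick line-traces to the target, smoothly rotates Base, and, once roughly aligned, spawns missiles at PuntoDeDisparo through a short Delay.
; A trace hit that is untagged or out of range clears the target and closes the gate.
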(event Custom|CloseGate
  (bind _base (Variables|Default|GetBase))
  (bind _base_2 (Variables|Default|GetBase))
  (bind _returnvalue (Transformation|GetWorldRotation _base_2))
  ;[1 1 1] Disparo mejorado. Busca a un objetivo, dibuja una traza hacia el y orienta el cañon. Spawnea el componente proyectil en la direccion del bicho seleccionado.
  (Transformation|SetWorldRotation _base (Transformation|GetWorldRotation _base) false false)
  (Utilities|FlowControl|Gate true) ; enters at Close
)

(event Custom|BuscarTarget
  (bind _base (Variables|Default|GetBase))
  (bind _returnvalue (Transformation|GetWorldRotation _base))
  ;[1 1 1] Disparo mejorado. Busca a un objetivo, dibuja una traza hacia el y orienta el cañon. Spawnea el componente proyectil en la direccion del bicho seleccionado.
  (bind _outhit (Collision|SphereTraceForObjects (Transformation|GetWorldLocation (Variables|Default|GetPuntoDeDisparo)) (Transformation|GetActorLocation) (Variables|Default|GetAlcance) (Utilities|Array|MakeArray "ObjectTypeQuery3") false (Utilities|Array|MakeArray 0) "None"))
  (Utilities|IsValid (.HitActor (Collision|BreakHitResult _outhit))
    (:Is%20Valid
      (if (Actor|ActorHasTag (.HitActor (Collision|BreakHitResult _outhit)) "Enemigo")
        (Utilities|IsValid (Variables|Default|GetTarget)
          (:Is%20Valid
            (Utilities|FlowControl|Gate true) ; enters at Open
          )
          (:Is%20Not%20Valid
            (Variables|Default|SetTarget (.HitActor (Collision|BreakHitResult _outhit)))
            (Utilities|FlowControl|Gate true) ; enters at Open
          ))))))

(event EventBeginPlay
  ;[1 1 1] Disparo mejorado. Busca a un objetivo, dibuja una traza hacia el y orienta el cañon. Spawnea el componente proyectil en la direccion del bicho seleccionado.
  (Utilities|Time|SetTimerbyFunctionName self "BuscarTarget" 0.2 true))

(event EventTick
  (params (DeltaSeconds :type Float%20%28single-precision%29))
  (bind _base (Variables|Default|GetBase))
  (bind _returnvalue (Transformation|GetWorldRotation _base))
  ;[1 1 1] Disparo mejorado. Busca a un objetivo, dibuja una traza hacia el y orienta el cañon. Spawnea el componente proyectil en la direccion del bicho seleccionado.
  (Utilities|FlowControl|Gate true
    (:Exit
      (Utilities|IsValid (Variables|Default|GetTarget)
        (:Is%20Valid
          (bind _outhit (Collision|LineTraceForObjects (Transformation|GetWorldLocation (Variables|Default|GetBase)) (Transformation|GetActorLocation (Variables|Default|GetTarget)) (Utilities|Array|MakeArray "ObjectTypeQuery3" "ObjectTypeQuery1") false 0 "None" true "(R=1.000000,G=0.000000,B=0.000000,A=1.000000)" "(R=0.000000,G=1.000000,B=0.000000,A=1.000000)" 0.5))
          (Utilities|IsValid (.HitActor (Collision|BreakHitResult _outhit))
            (:Is%20Valid
              (if (Actor|ActorHasTag (.HitActor (Collision|BreakHitResult _outhit)) "Enemigo")
                (if (<= (Transformation|GetDistanceTo (.HitActor (Collision|BreakHitResult _outhit)) self) (Variables|Default|GetAlcance))
                  (Transformation|SetWorldRotation (Variables|Default|GetBase) (Math|Interpolation|RInterpTo _returnvalue (Math|Rotator|FindLookatRotation (Transformation|GetWorldLocation _base) (Transformation|GetActorLocation (Variables|Default|GetTarget))) (Utilities|Time|GetWorldDeltaSeconds) (Variables|Default|GetVelocidad%20Rotacion%20Cabeza)) false false)
                  (if (Math|Rotator|Equal(Rotator) _returnvalue (Math|Rotator|FindLookatRotation (Transformation|GetWorldLocation _base) (Transformation|GetActorLocation (Variables|Default|GetTarget))) 6.0)
                    (Utilities|IsValid (.HitActor (Collision|BreakHitResult _outhit))
                      (:Is%20Valid
                        (Utilities|FlowControl|Delay 0.2)
                        (CallFunction|SpawnProjectile))
                      (:Is%20Not%20Valid
                        (Variables|Default|SetTarget 0))))
                  (else
                    (Variables|Default|SetTarget 0 :!label _label)
                    (CallFunction|CloseGate)))
                (else
                  (goto _label))))))
        (:Is%20Not%20Valid
          (CallFunction|BuscarTarget))))))

(fn ConstructionScript)

(fn SpawnProjectile
  (Game|SpawnActorfromClass "/Game/Assets/Level1/Blueprints/missile.missile_C" (Transformation|GetWorldTransform (Variables|Default|GetPuntoDeDisparo)) "Undefined" 0 0))