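; Homing missile projectile that damages tagged Bichito1 and Bichito2 enemies.
; Each tick it turns toward the first Bichito1 found in the world and resets its local-space projectile velocity to a fixed diagonal vector.
; Overlapping an "Enemigo" actor subtracts Damage from its Health; at zero or below, both enemy and missile are destroyed, so the missile survives non-lethal hits.
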(event EventBeginPlay)

(event EventTick
  (params (DeltaSeconds :type Float%20%28single-precision%29))
  (bind _self self)
  (bind _outactors (Actor|GetAllActorsOfClass "/Game/Prototipos/Level/Bichito1.Bichito1_C"))
  (Transformation|SetActorRotation _self (Math|Rotator|FindLookatRotation (Transformation|GetActorLocation _self) (Transformation|GetActorLocation (Utilities|Array|Get(acopy) _outactors))))
  (Game|Components|ProjectileMovement|SetVelocityinLocalSpace (Variables|Default|GetProjectileMovement) "100.000000,100.000000,100.000000"))

(event Collision|EventActorBeginOverlap
  (params (OtherActor :type Actor%20Object%20Reference))
  (if (Actor|ActorHasTag OtherActor "Enemigo")
    (bind _asbichito_1 (Utilities|Casting|CastToBichito1 OtherActor)
      (:then
        (Variables|/Game/Prototipos/Level/Bichito1.Bichito1_C|SetHealth _asbichito_1 (- (Variables|/Game/Prototipos/Level/Bichito1.Bichito1_C|GetHealth _asbichito_1) (Variables|Default|GetDamage)))
        (if (<= (Variables|/Game/Prototipos/Level/Bichito1.Bichito1_C|GetHealth _asbichito_1) 0.0)
          (Actor|DestroyActor _asbichito_1)
          (Actor|DestroyActor :!label _label)))
      (:CastFailed
        (bind _asbichito_2 (Utilities|Casting|CastToBichito2 OtherActor))
        (Variables|/Game/Prototipos/Level/Bichito2.Bichito2_C|SetHealth _asbichito_2 (- (Variables|/Game/Prototipos/Level/Bichito2.Bichito2_C|GetHealth _asbichito_2) (Variables|Default|GetDamage)))
        (if (<= (Variables|/Game/Prototipos/Level/Bichito2.Bichito2_C|GetHealth _asbichito_2) 0.0)
          (Actor|DestroyActor _asbichito_2)
          (goto _label))))))

(fn ConstructionScript)