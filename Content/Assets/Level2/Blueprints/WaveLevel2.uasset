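; Level 2 wave spawner that releases enemy critters (bichos) at its own location, one wave at a time.
; SpawnBichos or an expired countdown, ticked about once per second via a Delay on Tick, advances the wave until TotalOleadas and resets the timer.
; Each wave chains delayed loops through four Bichito types, with counts from per-type arrays indexed by wave.
; Every spawn increments BichosRestantes on the first Jugador found.
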(event Custom|SpawnBichos
  (if (< (Variables|Default|GetOleadaActual) (Variables|Default|GetTotalOleadas))
    (Variables|Default|SetOleadaActual (+ (Variables|Default|GetOleadaActual) 1))
    (Variables|Default|SetTimeOleada 30)
    (bind _index (Utilities|ForLoopwithDelay 0 (Utilities|Array|Get(acopy) (Variables|Default|GetBichosT1) (Variables|Default|GetOleadaActual)) 0.5)
      (:LoopBody
        (if (!= _index (Utilities|Array|Get(acopy) (Variables|Default|GetBichosT1) (Variables|Default|GetOleadaActual)))
          (AI|SpawnAIFromClass "/Game/Prototipos/Level/Bichito1.Bichito1_C" 0 (Transformation|GetActorLocation) "0, 0, 0" false)
          (bind _outactors (Actor|GetAllActorsOfClass "/Game/Prototipos/Level/Jugador.Jugador_C" :!label _label))
          (Variables|/Game/Prototipos/Level/Jugador.Jugador_C|SetBichosRestantes (Utilities|Array|Get(acopy) _outactors) (+ (Variables|/Game/Prototipos/Level/Jugador.Jugador_C|GetBichosRestantes (Utilities|Array|Get(acopy) _outactors)) 1))))
      (:Completed
        (bind _index_2 (Utilities|ForLoopwithDelay 0 (Utilities|Array|Get(acopy) (Variables|Default|GetBichosT2) (Variables|Default|GetOleadaActual)) 0.5)
          (:LoopBody
            (if (!= _index_2 (Utilities|Array|Get(acopy) (Variables|Default|GetBichosT2) (Variables|Default|GetOleadaActual)))
              (AI|SpawnAIFromClass "/Game/Prototipos/Level/Bichito2.Bichito2_C" 0 (Transformation|GetActorLocation) "0, 0, 0" false)
              (goto _label)))
          (:Completed
            (bind _index_3 (Utilities|ForLoopwithDelay 0 (Utilities|Array|Get(acopy) (Variables|Default|GetBichosT3) (Variables|Default|GetOleadaActual)) 0.5)
              (:LoopBody
                (if (!= _index_3 (Utilities|Array|Get(acopy) (Variables|Default|GetBichosT3) (Variables|Default|GetOleadaActual)))
                  (AI|SpawnAIFromClass "/Game/Prototipos/Level/Bichito3.Bichito3_C" 0 (Transformation|GetActorLocation) "0, 0, 0" false)
                  (goto _label)))
              (:Completed
                (bind _index_4 (Utilities|ForLoopwithDelay 0 (Utilities|Array|Get(acopy) (Variables|Default|GetBichosT4) (Variables|Default|GetOleadaActual)) 0.5)
                  (:LoopBody
                    (if (!= _index_4 (Utilities|Array|Get(acopy) (Variables|Default|GetBichosT4) (Variables|Default|GetOleadaActual)))
                      (AI|SpawnAIFromClass "/Game/Prototipos/Level/Bichito4.Bichito4_C" 0 (Transformation|GetActorLocation) "0, 0, 0" false)
                      (goto _label))))))))))))

(event EventTick
  (params (DeltaSeconds :type Float%20%28single-precision%29))
  (bind _bichost2 (Variables|Default|GetBichosT2))
  (bind _oleadaactual (Variables|Default|GetOleadaActual))
  (bind _oleadaactual_2 (Variables|Default|GetOleadaActual))
  (bind _bichost3 (Variables|Default|GetBichosT3))
  (bind _bichost4 (Variables|Default|GetBichosT4))
  (bind _bichost1 (Variables|Default|GetBichosT1))
  (bind _oleadaactual_3 (Variables|Default|GetOleadaActual))
  (bind _oleadaactual_4 (Variables|Default|GetOleadaActual))
  (bind _output (Utilities|Array|Get(acopy) _bichost4 _oleadaactual_4))
  (bind _output_2 (Utilities|Array|Get(acopy) _bichost1 _oleadaactual_3))
  (bind _output_3 (Utilities|Array|Get(acopy) _bichost2 _oleadaactual))
  (bind _output_4 (Utilities|Array|Get(acopy) _bichost3 _oleadaactual_2))
  (Utilities|FlowControl|Delay 1.0)
  (if (<= (Variables|Default|GetTimeOleada) 0)
    (if (< (Variables|Default|GetOleadaActual) (Variables|Default|GetTotalOleadas))
      (Math|Integer|IncrementInt (Variables|Default|GetOleadaActual)
        (:%20%20
          (Variables|Default|SetTimeOleada 30)
          (bind _index (Utilities|ForLoopwithDelay 0 _output_2 0.5)
            (:LoopBody
              (if (!= _index _output_2)
                (AI|SpawnAIFromClass "/Game/Prototipos/Level/Bichito1.Bichito1_C" 0 (Transformation|GetActorLocation) "0, 0, 0" false)
                (bind _outactors (Actor|GetAllActorsOfClass "/Game/Prototipos/Level/Jugador.Jugador_C" :!label _label))
                (Variables|/Game/Prototipos/Level/Jugador.Jugador_C|SetBichosRestantes (Utilities|Array|Get(acopy) _outactors) (+ (Variables|/Game/Prototipos/Level/Jugador.Jugador_C|GetBichosRestantes (Utilities|Array|Get(acopy) _outactors)) 1))))
            (:Completed
              (bind _index_2 (Utilities|ForLoopwithDelay 0 _output_3 0.5)
                (:LoopBody
                  (if (!= _index_2 _output_3)
                    (AI|SpawnAIFromClass "/Game/Prototipos/Level/Bichito2.Bichito2_C" 0 (Transformation|GetActorLocation) "0, 0, 0" false)
                    (goto _label)))
                (:Completed
                  (bind _index_3 (Utilities|ForLoopwithDelay 0 _output_4 0.5)
                    (:LoopBody
                      (if (!= _index_3 _output_4)
                        (AI|SpawnAIFromClass "/Game/Prototipos/Level/Bichito3.Bichito3_C" 0 (Transformation|GetActorLocation) "0, 0, 0" false)
                        (goto _label)))
                    (:Completed
                      (bind _index_4 (Utilities|ForLoopwithDelay 0 _output 0.5)
                        (:LoopBody
                          (if (!= _index_4 _output)
                            (AI|SpawnAIFromClass "/Game/Prototipos/Level/Bichito4.Bichito4_C" 0 (Transformation|GetActorLocation) "0, 0, 0" false)
                            (goto _label)))))))))))))
    (else
      (Variables|Default|SetTimeOleada (- (Variables|Default|GetTimeOleada) 1)))))

(fn ConstructionScript)